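; BP_Blocks is a grid of breakable blocks that react to BP_Ball hits.
; The Construction Script builds the grid from static mesh components, using X, Y and Padding for count and spacing.
; A ball hit swaps a block from BasicMaterial to HitMaterial, using the material as its damage state.
; A further hit destroys that component, with a coin-flip chance to spawn a speed or new-ball bonus in its place.
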(event `self.ReceiveHit`
  (params (MyComp :type "PrimitiveComponent Object Reference") (Other :type "Actor Object Reference") (OtherComp :type "PrimitiveComponent Object Reference") (bSelfMoved :type Boolean) (HitLocation :type "Vector Structure") (HitNormal :type "Vector Structure") (NormalImpulse :type "Vector Structure") (Hit :type "HitResult Structure (by ref)"))
  (bind (_returnvalue_x _returnvalue_y _returnvalue_z) (`KismetMathLibrary.BreakVector` (`SceneComponent.K2_GetComponentLocation` MyComp)))
  (cast `/Game/MyGame/Blueprints/BP_Ball` Other)
  (if (== (`PrimitiveComponent.GetMaterial` MyComp 0) (`self.BasicMaterial`))
    (`PrimitiveComponent.SetMaterial` MyComp 0 (`self.HitMaterial`))
    (elif (`KismetMathLibrary.RandomBool`)
      (`|SpawnActorFromClass` (select `int` (`KismetMathLibrary.RandomIntegerInRange` 0 1) :`0` "/Game/MyGame/Blueprints/BP_BonusSpeed.BP_BonusSpeed_C" :`1` "/Game/MyGame/Blueprints/BP_BonusNewBall.BP_BonusNewBall_C" :!type "Actor Class Reference") (`KismetMathLibrary.MakeTransform` (`KismetMathLibrary.MakeVector` _returnvalue_x _returnvalue_y _returnvalue_z)) "AlwaysSpawn" "OverrideRootScale" null null)
      (`ActorComponent.K2_DestroyComponent` MyComp)
      (else
        (`ActorComponent.K2_DestroyComponent` MyComp)))))

(fn `UserConstructionScript`
  (for _index (range (+ (`self.x`) 1))
    (for _index_2 (range (+ (`self.y`) 1))
      (`AddComponent|NODE_AddStaticMeshComponent-0` :`RelativeTransform` (`KismetMathLibrary.MakeTransform` (`KismetMathLibrary.MakeVector` (`KismetMathLibrary.Conv_IntToDouble` (* (`self.Padding`) _index)) (`KismetMathLibrary.Conv_IntToDouble` (* _index_2 (`self.Padding`)))))))))