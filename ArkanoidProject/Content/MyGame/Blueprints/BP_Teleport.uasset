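; Teleport pad actor that turns gold and opens a WBP_TeleportControll widget with mouse cursor while a ThirdPersonCharacter overlaps it.
; Its Teleport event spends the character's energy and moves it near GetNextDestination's actor, advancing a counter on success.
; Landing scatter shrinks as spent energy rises, via a clamped range mapping.
; GetNextDestination's round-robin lookup into Destinations appears unconnected in the graph.
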(event `self.ReceiveActorBeginOverlap`
  (params (OtherActor :type "Actor Object Reference"))
  (bind _returnvalue (`GameplayStatics.GetPlayerController` 0))
  (bind _asthird_person_character (cast `/Game/ThirdPersonBP/Blueprints/ThirdPersonCharacter` OtherActor))
  (set `self.Character` _asthird_person_character)
  (`PrimitiveComponent.SetMaterial` (`self.Surface`) 0 "/Game/StarterContent/Materials/M_Metal_Gold.M_Metal_Gold")
  (bind _returnvalue_2 (`|CreateWidget` "/Game/ThirdPersonBP/Blueprints/WBP_TeleportControll.WBP_TeleportControll_C" null self))
  (bind _output_get (set `self.Widget` _returnvalue_2))
  (`UserWidget.AddToViewport` _output_get 0)
  (`WidgetBlueprintLibrary.SetInputMode_GameAndUIEx` _returnvalue _output_get)
  (set `PlayerController.bShowMouseCursor` true _returnvalue))

(event `self.ReceiveActorEndOverlap`
  (params (OtherActor :type "Actor Object Reference"))
  (bind _returnvalue (`GameplayStatics.GetPlayerController` 0))
  (cast `/Game/ThirdPersonBP/Blueprints/ThirdPersonCharacter` OtherActor)
  (set `self.Character` null)
  (`PrimitiveComponent.SetMaterial` (`self.Surface`) 0 "/Game/StarterContent/Materials/M_Metal_Burnished_Steel.M_Metal_Burnished_Steel")
  (`Widget.RemoveFromParent` (`self.Widget`))
  (`WidgetBlueprintLibrary.SetInputMode_GameOnly` _returnvalue)
  (set `PlayerController.bShowMouseCursor` false _returnvalue))

(event `Teleport`
  (bind _output (`self.GetNextDestination`))
  (bind _character (`self.Character`))
  (`/Engine/EditorBlueprintResources/StandardMacros.IsValid` _character
    (:`Is Valid`
      (if (> (`/Game/ThirdPersonBP/Blueprints/ThirdPersonCharacter.GetEnergy` _character) 0.0)
        (`/Engine/EditorBlueprintResources/StandardMacros.IsValid` _output
          (:`Is Valid`
            (bind _spentenergy1 (`/Game/ThirdPersonBP/Blueprints/ThirdPersonCharacter.SpendEnergy` (`self.Character`)))
            (bind _returnvalue (`KismetMathLibrary.MapRangeClamped` _spentenergy1 0.0 1.0 200.0))
            (bind _returnvalue_2 (`self.K2_TeleportTo` :`self` (`self.Character`) :`DestLocation` (`KismetMathLibrary.RandomPointInBoundingBox` (`self.K2_GetActorLocation` _output) (`KismetMathLibrary.MakeVector` _returnvalue _returnvalue))))
            (if _returnvalue_2
              (`/Engine/EditorBlueprintResources/StandardMacros.IncrementInt` (`self.Counter`)))))))))

(fn `UserConstructionScript`)