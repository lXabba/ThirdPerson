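; Player pawn that moves sideways from player input and owns a ball, apparently as a paddle.
; BeginPlay sets game-only input and spawns a BP_Ball at the capsule, binding an event to its OnDead dispatcher.
; MoveRight applies a swept Y-axis offset scaled by Speed and delta time.
; Hitting a BP_BonusNewBall adds to Speed, while any other hit resets it to BaseSpeed.
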(event `self.ReceiveBeginPlay`
  (`|ExecutionSequence`
    (:`then_0`
      (`WidgetBlueprintLibrary.SetInputMode_GameOnly` (`GameplayStatics.GetPlayerController` 0)))
    (:`then_1`
      (`self.SpawnBall`))))

(event `InputAxis|MoveRight`
  (params (AxisValue :type "Float (single-precision)"))
  (`self.K2_AddActorWorldOffset` (`KismetMathLibrary.MakeVector` 0.0 (* AxisValue (`GameplayStatics.GetWorldDeltaSeconds`) (`self.Speed`))) true))

(event `self.ReceiveHit`
  (params (MyComp :type "PrimitiveComponent Object Reference") (Other :type "Actor Object Reference") (OtherComp :type "PrimitiveComponent Object Reference") (bSelfMoved :type Boolean) (HitLocation :type "Vector Structure") (HitNormal :type "Vector Structure") (NormalImpulse :type "Vector Structure") (Hit :type "HitResult Structure (by ref)"))
  (cast `/Game/MyGame/Blueprints/BP_BonusNewBall` Other
    (:`then`
      (set `self.Speed` (+ (`self.Speed`) 500.0)))
    (:`CastFailed`
      (set `self.Speed` (`self.BaseSpeed`)))))

(fn `SpawnBall`
  (bind _returnvalue (`|SpawnActorFromClass` "/Game/MyGame/Blueprints/BP_Ball.BP_Ball_C" (`KismetMathLibrary.MakeTransform` (`SceneComponent.K2_GetComponentLocation` (`self.Capsule`))) "AlwaysSpawn" "OverrideRootScale" null null))
  (bind _output_get (set `self.PlayingBall` _returnvalue))
  (add `/Game/MyGame/Blueprints/BP_Ball.OnDead` _output_get (`|CreateDelegate` :!event `SpawnBall`))
  (return))

(fn `UserConstructionScript`)